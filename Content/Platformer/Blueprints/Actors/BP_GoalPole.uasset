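; BP_GoalPole is the platformer's goal pole, running a timed end-of-level sequence on the character while its flag moves to an end point.
; The character moves through two points with jump and fall animations, then explodes and is hidden.
; AddTimePoints counts the remaining level time down into points.
; If the time's last digit matches FireworkShowSpecialNumber, that many bonus-point fireworks follow at random spots in a box.
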(event `self.RunGoalPoleLogic`
  (params (Character :type "PFCharacter Object Reference"))
  (bind _playerendpoint (`self.PlayerEndPoint`))
  (bind _capsulecomponent (`Character.CapsuleComponent` Character))
  (bind _fireworksareacollision (`self.FireworksAreaCollision`))
  (bind _flagendpoint (`self.FlagEndPoint`))
  (bind _mesh (`Character.Mesh` Character))
  (bind _playerexplodepoint (`self.PlayerExplodePoint`))
  (bind _returnvalue (`SceneComponent.K2_GetComponentLocation` _capsulecomponent))
  (`KismetSystemLibrary.Delay` 1.0)
  (`GameplayStatics.PlaySound2D` (`self.SoundEffect`) 1.0 1.0 0.0 null null)
  (`|ExecutionSequence`
    (:`then_0`
      (`KismetSystemLibrary.MoveComponentTo` (`Character.CapsuleComponent` Character) (`SceneComponent.K2_GetComponentLocation` _playerendpoint) (`SceneComponent.K2_GetComponentRotation` _playerendpoint) false false 1.0)
      (`SkeletalMeshComponent.PlayAnimation` _mesh "/Game/Characters/Mannequins/Animations/Manny/MM_Jump.MM_Jump" false)
      (`KismetSystemLibrary.Delay` 0.3)
      (`SkeletalMeshComponent.PlayAnimation` _mesh "/Game/Characters/Mannequins/Animations/Manny/MM_Fall_Loop.MM_Fall_Loop" true)
      (`KismetSystemLibrary.MoveComponentTo` (`Character.CapsuleComponent` Character) (`SceneComponent.K2_GetComponentLocation` _playerexplodepoint) (`SceneComponent.K2_GetComponentRotation` _playerexplodepoint) false false 0.5)
      ;[0.3497 0 1 1 16] Explode the player
      (`GameplayStatics.PlaySoundAtLocation` (`self.CharacterExplosionSoundEffect`) _returnvalue (struct) 1.0 1.0 0.0 null null null null)
      (`GameplayStatics.SpawnEmitterAtLocation` (`self.CharacterExplosionParticleEffect`) _returnvalue (struct) (2.0 2.0 2.0))
      (`SceneComponent.SetVisibility` _capsulecomponent false true)
      (bind _asbp_player_controller (cast `/Game/Platformer/Blueprints/Player/BP_PlayerController` (`Pawn.GetController` Character)))
      (if (== (`self.FireworkShowSpecialNumber`) (`KismetStringLibrary.Right` (`KismetStringLibrary.Conv_IntToString` (`PFPlayerController.GetLevelTime` _asbp_player_controller)) 1))
        (`self.AddTimePoints` Character
          (:`Out`
            (`KismetSystemLibrary.Delay` 0.5 :!label _label)
            (`/Engine/EditorBlueprintResources/StandardMacros.Do N` (`self.FireworkShowSpecialNumber`)
              (:`Exit`
                (bind _output_get (set `self.FireworkLocale` (`KismetMathLibrary.RandomPointInBoundingBox` (`SceneComponent.K2_GetComponentLocation` _fireworksareacollision) (`BoxComponent.BoxExtent` _fireworksareacollision))))
                (`GameplayStatics.PlaySoundAtLocation` (`self.FireworkSoundEffect`) _output_get (struct) 1.0 1.0 0.0 null null null null)
                (`GameplayStatics.SpawnEmitterAtLocation` (`self.FireworkParticleEffect`) _output_get (struct) (10.0 10.0 10.0))
                (message `PlayerInterface.AddToPoints` Character (`self.FireworkPoints`))
                (goto _label)))))
        (else
          (`self.AddTimePoints` Character))))
    (:`then_1`
      (`KismetSystemLibrary.MoveComponentTo` (`self.Flag`) (`SceneComponent.RelativeLocation` _flagendpoint) (`SceneComponent.RelativeRotation` _flagendpoint) false false 1.0))))

(fn `UserConstructionScript`)