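; BP_SimpleCoin is a self-running coin effect that animates on spawn, then removes itself, with no collision or scoring logic in its graphs.
; On BeginPlay, CoinTimeline drives the mesh's relative height and yaw at a fixed tilt.
; When the timeline finishes, it spawns the P_Loot_Pickup particle at the mesh's world location and destroys the actor.
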(event `self.ReceiveBeginPlay`
  (`TimelineComponent.SetPlayRate` (`self.CoinTimeline`) 1.0)
  (bind (_direction _movement _rotation) (`Timeline|CoinTimeline` :!via `PlayFromStart`)
    (:`Update`
      (`SceneComponent.K2_SetRelativeLocationAndRotation` (`self.CoinMesh`) (`KismetMathLibrary.MakeVector` 0.0 0.0 _movement) (`KismetMathLibrary.MakeRotator` -70.0 -90.0 _rotation) false false))
    (:`Finished`
      (`GameplayStatics.SpawnEmitterAtLocation` "/Game/InfinityBladeEffects/Effects/FX_Treasure/Loot/P_Loot_Pickup.P_Loot_Pickup" (`SceneComponent.K2_GetComponentLocation` (`self.CoinMesh`)))
      (`self.K2_DestroyActor`))))

(fn `UserConstructionScript`)