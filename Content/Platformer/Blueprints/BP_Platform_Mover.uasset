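; BP_Platform_Mover is a moving one-way platform for a platformer.
; On BeginPlay, a timeline at a configurable play rate lerps the Platform component between start and end relative locations without sweeping.
; A bottom trigger disables the platform's collision while the player overlaps it, letting them pass through from below.
; A top trigger messages overlapping actors with a reference to the platform, then clears it on exit.
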(event `self.CollisionBottom.OnComponentBeginOverlap`
  (params (OverlappedComponent :type "PrimitiveComponent Object Reference") (OtherActor :type "Actor Object Reference") (OtherComp :type "PrimitiveComponent Object Reference") (OtherBodyIndex :type Integer) (bFromSweep :type Boolean) (SweepResult :type "HitResult Structure (by ref)"))
  (if (== OtherActor (`GameplayStatics.GetPlayerCharacter` 0))
    (`PrimitiveComponent.SetCollisionEnabled` (`self.Platform`) "NoCollision")))

(event `self.CollisionBottom.OnComponentEndOverlap`
  (params (OverlappedComponent :type "PrimitiveComponent Object Reference") (OtherActor :type "Actor Object Reference") (OtherComp :type "PrimitiveComponent Object Reference") (OtherBodyIndex :type Integer))
  (if (== OtherActor (`GameplayStatics.GetPlayerCharacter` 0))
    (`PrimitiveComponent.SetCollisionEnabled` (`self.Platform`) "QueryAndPhysics")))

(event `self.CollisionTop.OnComponentBeginOverlap`
  (params (OverlappedComponent :type "PrimitiveComponent Object Reference") (OtherActor :type "Actor Object Reference") (OtherComp :type "PrimitiveComponent Object Reference") (OtherBodyIndex :type Integer) (bFromSweep :type Boolean) (SweepResult :type "HitResult Structure (by ref)"))
  (message `PlayerInterface.UpdateOverlappingPlatform` OtherActor self))

(event `self.CollisionTop.OnComponentEndOverlap`
  (params (OverlappedComponent :type "PrimitiveComponent Object Reference") (OtherActor :type "Actor Object Reference") (OtherComp :type "PrimitiveComponent Object Reference") (OtherBodyIndex :type Integer))
  (message `PlayerInterface.UpdateOverlappingPlatform` OtherActor null))

(event `self.ReceiveBeginPlay`
  (`TimelineComponent.SetPlayRate` (`self.PlatformMovement`) (`self.PlayRate`))
  (bind (_direction _movement) (`Timeline|PlatformMovement`)
    (:`Update`
      (`SceneComponent.K2_SetRelativeLocation` (`self.Platform`) (`KismetMathLibrary.VLerp` (`self.Loc_Start`) (`self.Loc_End`) _movement) false false))))

(fn `UserConstructionScript`)