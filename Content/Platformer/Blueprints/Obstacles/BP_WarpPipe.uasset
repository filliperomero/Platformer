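; Warp pipe obstacle for a platformer that animates a character into the pipe and out at a warp destination.
; AnimateCharacter picks an entry timeline by IsPipeDown and offsets the character's capsule in Z from WarpInPoint.
; After a short delay and a sound, both paths share an exit branch on IsPipeExitDown, whose timelines move the capsule in Z from WarpToLocation.
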(event `self.AnimateCharacter`
  (params (Character :type "PFCharacter Object Reference"))
  (if (`self.bIsPipeDown`)
    (bind (_direction _movement) (`Timeline|IntoDownPipe` :!via `PlayFromStart`)
      (:`Update`
        (`SceneComponent.K2_SetRelativeLocation` (`Character.CapsuleComponent` Character) (`KismetMathLibrary.MakeVector` (.x (`SceneComponent.K2_GetComponentLocation` (`self.WarpInPoint`))) (.y (`SceneComponent.K2_GetComponentLocation` (`self.WarpInPoint`))) (+ _movement (.z (`SceneComponent.K2_GetComponentLocation` (`self.WarpInPoint`))))) false false))
      (:`Finished`
        (`KismetSystemLibrary.Delay` 0.4)
        (`GameplayStatics.PlaySound2D` (`self.SoundEffect`) 1.0 1.0 0.0 null null)
        (if (`self.bIsPipeExitDown`) :!label _label
          (bind (_direction_2 _movement_2) (`Timeline|RisingUpOutOfPipe` :!via `PlayFromStart`)
            (:`Update`
              (`SceneComponent.K2_SetRelativeLocation` (`Character.CapsuleComponent` Character) (`KismetMathLibrary.MakeVector` (.x (`self.WarpToLocation`)) (.y (`self.WarpToLocation`)) (+ _movement_2 (.z (`self.WarpToLocation`)))) false false)))
          (else
            (bind (_direction_3 _movement_3) (`Timeline|Timeline_0` :!via `PlayFromStart`)
              (:`Update`
                (`SceneComponent.K2_SetRelativeLocation` (`Character.CapsuleComponent` Character) (`KismetMathLibrary.MakeVector` (.x (`self.WarpToLocation`)) (.y (`self.WarpToLocation`)) (+ _movement_3 (.z (`self.WarpToLocation`)))) false false)))))))
    (else
      (bind (_direction_4 _movement_4) (`Timeline|Timeline` :!via `PlayFromStart`)
        (:`Update`
          (`SceneComponent.K2_SetRelativeLocation` (`Character.CapsuleComponent` Character) (`KismetMathLibrary.MakeVector` (.x (`SceneComponent.K2_GetComponentLocation` (`self.WarpInPoint`))) (.y (`SceneComponent.K2_GetComponentLocation` (`self.WarpInPoint`))) (+ _movement_4 (.z (`SceneComponent.K2_GetComponentLocation` (`self.WarpInPoint`))))) false false))
        (:`Finished`
          (`KismetSystemLibrary.Delay` 0.4)
          (`GameplayStatics.PlaySound2D` (`self.SoundEffect`) 1.0 1.0 0.0 null null)
          (goto _label))))))

(fn `UserConstructionScript`)