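; Mushroom jump pad for the platformer that launches player characters who land on its top.
; A hit on MushroomTop from a PlayerInterface actor with a straight-down impact normal passes a DoOnce gate and launches the character by LaunchVelocity.
; The launch spawns a leap particle burst at the impact point and plays a timeline that scales the mushroom top.
; Timeline updates trigger a short delay before ResetLauncher reopens the gate.
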(event `ResetLauncher`
  (goto _label :!via `Reset`))

(event `self.MushroomTop.OnComponentHit`
  (params (HitComponent :type "PrimitiveComponent Object Reference") (OtherActor :type "Actor Object Reference") (OtherComp :type "PrimitiveComponent Object Reference") (NormalImpulse :type "Vector Structure") (Hit :type "HitResult Structure (by ref)"))
  (bind (_bblockinghit _binitialoverlap _time _distance _location _impactpoint _normal _impactnormal) (`GameplayStatics.BreakHitResult` Hit))
  (if (and (`KismetSystemLibrary.DoesImplementInterface` OtherActor "/Script/Platformer.PlayerInterface") (`KismetMathLibrary.EqualExactly_VectorVector` _impactnormal (0.0 0.0 -1.0)))
    (`/Engine/EditorBlueprintResources/StandardMacros.DoOnce` false :!label _label
      (:`Completed`
        (message `PlayerInterface.LaunchCharacter` OtherActor (`self.LaunchVelocity`))
        (`GameplayStatics.SpawnEmitterAtLocation` "/Game/InfinityBladeEffects/Effects/FX_Skill_Leap/P_Skill_Leap_Base_Launch.P_Skill_Leap_Base_Launch" _impactpoint (struct) (3.0 3.0 3.0))
        (bind (_direction _scale_multipler) (`Timeline|Timeline` :!via `PlayFromStart`)
          (:`Update`
            (bind _returnvalue (* _scale_multipler (`self.MushroomTopScaleXY`)))
            (`SceneComponent.SetRelativeScale3D` (`self.MushroomTop`) (`KismetMathLibrary.MakeVector` _returnvalue _returnvalue (* _scale_multipler (`self.MushroomTopScaleZ`))))
            (`KismetSystemLibrary.Delay` 0.2)
            (`self.ResetLauncher`)))))))

(fn `UserConstructionScript`)